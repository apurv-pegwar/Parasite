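; BP_Enemy is an enemy that chases the player character while overlapping it and plays an attack montage on reaching it.
; AI MoveTo success triggers the montage behind a timed CanAttack cooldown, re-issuing the chase during cooldown or after the montage if still in range.
; Ending overlap halts movement.
; Player contact with its Box shows the BP_START widget and mouse cursor, then destroys the enemy after a short delay.
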(event OnComponentBeginOverlap(Box)
  (params (OverlappedComponent :type Primitive%20Component%20Object%20Reference) (OtherActor :type Actor%20Object%20Reference) (OtherComp :type Primitive%20Component%20Object%20Reference) (OtherBodyIndex :type Integer) (bFromSweep :type Boolean) (SweepResult :type Hit%20Result%20Structure%20%28by%20ref%29))
  (Utilities|Casting|CastToBP_MyCharacter OtherActor)
  (bind _returnvalue (UserInterface|CreateWidget "/Game/BluePrints/BP_START.BP_START_C"))
  (UserInterface|Viewport|AddtoViewport _returnvalue 0)
  (Variables|/Script/Engine.PlayerController|SetbShowMouseCursor (Game|GetPlayerController 0) true)
  (Utilities|FlowControl|Delay 0.2)
  (Actor|DestroyActor))

(event Custom|Chase%20the%20players
  (AI|AIMoveTo self "0, 0, 0" (Game|GetPlayerCharacter 0) 1e+02 false
    (:OnSuccess
      (if (Variables|Default|GetCanAttack)
        (Variables|Default|SetCanAttack false)
        (Animation|Montage|PlayMontage (Variables|Character|GetMesh) 0
          (:then
            (Utilities|FlowControl|Delay (Variables|Default|GetAttackRate))
            (Variables|Default|SetCanAttack true))
          (:OnCompleted
            (if (Variables|Default|GetPlayerInrange)
              (CallFunction|ChasethePlayers))))
        (else
          (CallFunction|ChasethePlayers))))))

(event Collision|EventActorBeginOverlap
  (params (OtherActor :type Actor%20Object%20Reference))
  (Utilities|Casting|CastToBP_MyCharacter OtherActor)
  (Variables|Default|SetPlayerInrange true)
  (CallFunction|ChasethePlayers))

(event Collision|EventActorEndOverlap
  (params (OtherActor :type Actor%20Object%20Reference))
  (Utilities|Casting|CastToBP_MyCharacter OtherActor)
  (Variables|Default|SetPlayerInrange false)
  (Components|Movement|StopMovementImmediately (Variables|Character|GetCharacterMovement)))

(fn ConstructionScript)
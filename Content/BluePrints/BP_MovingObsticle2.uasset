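; BP_MovingObsticle2 is a moving obstacle that shuttles between two arrow-component markers and reacts when the player character touches it.
; Tick moves it at constant MovementSpeed, flipping the target on arrival; the random-speed node is never run.
; Overlapping BP_MyCharacter shows the BP_START widget and mouse cursor, then destroys the obstacle itself after a short delay.
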(event EventBeginPlay
  (Variables|Default|SetCurrentLocation (Transformation|GetActorLocation))
  (Variables|Default|SetStartPointLocation (Transformation|GetWorldLocation (Variables|Default|GetStart%20Arrow)))
  (Variables|Default|SetEndPointLocation (Transformation|GetWorldLocation (Variables|Default|GetEnd%20Arrow1)))
  (if (Variables|Default|GetMoveToStartPoint)
    (Variables|Default|SetTargetLocation (Variables|Default|GetStartPointLocation))
    (else
      (Variables|Default|SetTargetLocation (Variables|Default|GetEndPointLocation)))))

(event Collision|EventActorBeginOverlap
  (params (OtherActor :type Actor%20Object%20Reference))
  (Utilities|Casting|CastToBP_MyCharacter OtherActor)
  (bind _returnvalue (UserInterface|CreateWidget "/Game/BluePrints/BP_START.BP_START_C"))
  (UserInterface|Viewport|AddtoViewport _returnvalue 0)
  (Variables|/Script/Engine.PlayerController|SetbShowMouseCursor (Game|GetPlayerController 0) true)
  (Utilities|FlowControl|Delay 0.2)
  (Actor|DestroyActor))

(event EventTick
  (params (DeltaSeconds :type Float%20%28single-precision%29))
  (Variables|Default|SetFrametime DeltaSeconds)
  (bind _output_get (Variables|Default|SetCurrentLocation (Math|Interpolation|VInterptoConstant (Variables|Default|GetCurrentLocation) (Variables|Default|GetTargetLocation) (Variables|Default|GetFrametime) (Variables|Default|GetMovementSpeed))))
  (Transformation|SetActorLocation _output_get false false)
  (if (<= (Math|Vector|VectorLength (- (Transformation|GetActorLocation) (Variables|Default|GetTargetLocation))) 0.0)
    (if (Variables|Default|GetMoveToStartPoint)
      (Variables|Default|SetTargetLocation (Variables|Default|GetEndPointLocation))
      (Variables|Default|SetMoveToStartPoint false)
      (else
        (Variables|Default|SetTargetLocation (Variables|Default|GetStartPointLocation))
        (Variables|Default|SetMoveToStartPoint true)))))

(fn ConstructionScript)